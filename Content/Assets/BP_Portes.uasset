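; BP_Portes is an automatic door that moves along Z when a ThirdPersonCharacter enters its Box trigger.
; Begin overlap plays Timeline_1 to drive PorteMoving's relative Z, posting the Wwise open sound only when exactly one character is inside.
; End overlap reverses the timeline and posts the close sound once the box is empty.
; An older DoOnce-gated version using Timeline_0 remains disconnected and never runs.
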(event `self.ReceiveTick`
  (params (DeltaSeconds :type "Float (single-precision)"))
  ;[1 1 1] A VOMIR
)

(event `self.Box.OnComponentBeginOverlap`
  (params (OverlappedComponent :type "PrimitiveComponent Object Reference") (OtherActor :type "Actor Object Reference") (OtherComp :type "PrimitiveComponent Object Reference") (OtherBodyIndex :type Integer) (bFromSweep :type Boolean) (SweepResult :type "HitResult Structure (by ref)"))
  (bind _returnvalue (`KismetArrayLibrary.Array_Length` (`PrimitiveComponent.GetOverlappingActors` (`self.Box`) "/Game/Blueprints/ThirdPersonCharacter.ThirdPersonCharacter_C")))
  (if (> _returnvalue 0)
    (if (== _returnvalue 1)
      (`AkGameplayStatics.PostEvent` "/Game/Audio/Event_Amb/Play_Open_Door_SFX.Play_Open_Door_SFX" self)
      (bind (_direction _movement) (`Timeline|Timeline_1` :!label _label)
        (:`Update`
          (`SceneComponent.K2_SetRelativeLocation` (`self.Porte_Moving`) (`KismetMathLibrary.MakeVector` 0.0 0.0 _movement) false false)))
      (else
        (goto _label)))))

(event `self.Box.OnComponentEndOverlap`
  (params (OverlappedComponent :type "PrimitiveComponent Object Reference") (OtherActor :type "Actor Object Reference") (OtherComp :type "PrimitiveComponent Object Reference") (OtherBodyIndex :type Integer))
  (if (<= (`KismetArrayLibrary.Array_Length` (`PrimitiveComponent.GetOverlappingActors` (`self.Box`) "/Game/Blueprints/ThirdPersonCharacter.ThirdPersonCharacter_C")) 0)
    (`AkGameplayStatics.PostEvent` "/Game/Audio/Event_Amb/Play_Close_Door_SFX.Play_Close_Door_SFX" self)
    (goto _label :!via `Reverse`)))

(fn `UserConstructionScript`)