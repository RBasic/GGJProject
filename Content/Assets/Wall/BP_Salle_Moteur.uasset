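; BP_Salle_Moteur is an engine room Blueprint that populates itself with randomized objects when play begins.
; BeginPlay passes SharedRoot to FindLocationsForSpawn, spawns a BP_Object slightly above each returned location and randomizes its type.
; An unconnected chain that would spawn one BP_Placement at a random location and set its system type and object to place never runs.
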(event `self.ReceiveBeginPlay`
  (`|ExecutionSequence`
    (:`then_0`
      (bind _newparam (`/Game/Blueprints/MyFonctionLibrary.Find_Locations_For_Spawn` (`self.SharedRoot`) -1))
      (for _array_element _newparam
        (bind _returnvalue (`|SpawnActorFromClass` "/Game/Blueprints/BP_Object.BP_Object_C" (`KismetMathLibrary.MakeTransform` (+ _array_element (0.0 0.0 70.0))) "Undefined" "OverrideRootScale" null null))
        (`/Game/Blueprints/BP_Object.Randomize_Object_Type` _returnvalue)))))

(fn `UserConstructionScript`)