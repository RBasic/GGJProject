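; BP_Cockpit is a cockpit actor whose Blueprint currently does nothing at runtime, as BeginPlay and the construction script are empty.
; Three disconnected chains remain, each getting points from FindLocationsForSpawn on the scene root and spawning slightly above them.
; Two spawn BP_Object at every point, one also randomizing its type.
; The third spawns one BP_Placement at a random point and sets its system type and object to place.
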(event `self.ReceiveBeginPlay`)

(fn `UserConstructionScript`)