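; BP_Salon is a salon Blueprint whose object-spawning logic is disconnected, so BeginPlay and the construction script do nothing.
; One unused chain spawns a BP_Object slightly above each location returned by FindLocationsForSpawn and randomizes its type.
; A second unused chain spawns one BP_Placement at a randomly picked location and sets its system type and object to place.
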(event `self.ReceiveBeginPlay`)

(fn `UserConstructionScript`)