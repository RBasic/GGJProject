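; Grabbable physics prop that the construction script randomly makes either a ready-to-use tool with a name widget or a damaged part needing repair.
; While repairing, Tick fills a progress bar and swaps meshes at half and full progress, re-grabbing through the player's physics handle after each swap.
; Start and stop repair drive Wwise tool sounds switched by required tool type.
; Respawn waits briefly, clears velocity and teleports to the spawn origin.
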(event `self.ReceiveBeginPlay`
  (set `self.Origin` (`self.K2_GetActorLocation`))
  (if (`self.Repaired?`)
    (`self.SwitchMesh` 2)
    (`ActorComponent.K2_DestroyComponent` (`self.WG_ProgressBar`))
    (bind _aswg_tool_text (cast `/Game/Widgets/WG_ToolText` (`WidgetComponent.GetUserWidgetObject` (`self.WG_ToolText`))))
    (`TextBlock.SetText` (`/Game/Widgets/WG_ToolText.ToolName` _aswg_tool_text) (`KismetTextLibrary.Conv_StringToText` (`|GetEnumeratorNameAsString` (`self.ObjectType`))))
    (else
      (`self.SwitchMesh` 0)
      (bind _aswg_repair_progress_bar (cast `/Game/Widgets/WG_RepairProgressBar` (`WidgetComponent.GetUserWidgetObject` (`self.WG_ProgressBar`))))
      (set `self.ProgressBar` (`/Game/Widgets/WG_RepairProgressBar.RepairProgress` _aswg_repair_progress_bar)))))

(event `self.ReceiveTick`
  (params (DeltaSeconds :type "Float (single-precision)"))
  (bind _staticmesh (`self.StaticMesh`))
  (bind _playergrabberref (`self.PlayerGrabberRef`))
  (if (not (`self.Repaired?`))
    (`|ExecutionSequence`
      (:`then_0`
        (if (`self.Repairing?`)
          (bind _output_get (set `self.RepairingProgress` (+ (* DeltaSeconds (`self.RepairSpeed`)) (`self.RepairingProgress`))))
          (`ProgressBar.SetPercent` (`self.ProgressBar`) _output_get)))
      (:`then_1`
        (if (>= (`self.RepairingProgress`) 1.0)
          (`/Engine/EditorBlueprintResources/StandardMacros.DoOnce` false
            (:`Completed`
              (`self.SwitchMesh` 2)
              (`ActorComponent.K2_DestroyComponent` (`self.WG_ProgressBar`))
              (`self.StopRepair`)
              (set `self.Repaired?` true)
              (`/Engine/EditorBlueprintResources/StandardMacros.IsValid` _playergrabberref :!label _label
                (:`Is Valid`
                  (`PhysicsHandleComponent.GrabComponentAtLocation` (`/Game/Blueprints/ThirdPersonCharacter.PhysicsHandle` _playergrabberref) _staticmesh "None" (`PrimitiveComponent.GetCenterOfMass` _staticmesh "None"))))))
          (elif (>= (`self.RepairingProgress`) 0.5)
            (`/Engine/EditorBlueprintResources/StandardMacros.DoOnce` false
              (:`Completed`
                (`self.SwitchMesh` 1)
                (goto _label)))))))))

(event `SwitchMesh`
  (params (Index :type Integer))
  (`StaticMeshComponent.SetStaticMesh` (`self.StaticMesh`) (`|GetArrayItem` (`self.Meshes`) Index))
  (set `self.IndexMesh` Index))

(event `StartRepair`
  (if (not (`self.Repaired?`))
    (set `self.Repairing?` true)
    (`AkGameplayStatics.SetSwitch` "Tools" (`KismetStringLibrary.Conv_StringToName` (`KismetStringLibrary.Replace` (`|GetEnumeratorNameAsString` (`self.RepairObject`)) " " "_")) self)
    (`AkGameplayStatics.PostEvent` "/Game/Audio/Switch_Play_Tools.Switch_Play_Tools" self)))

(event `StopRepair`
  (set `self.Repairing?` false)
  (`AkGameplayStatics.PostEvent` "/Game/Audio/Switch_Stop_Tools.Switch_Stop_Tools" self))

(event `Respawn`
  (bind _staticmesh (`self.StaticMesh`))
  (`KismetSystemLibrary.Delay` 2.0)
  (`PrimitiveComponent.SetAllPhysicsAngularVelocityInDegrees` _staticmesh (0.0 0.0 0.0) false)
  (`PrimitiveComponent.SetAllPhysicsLinearVelocity` _staticmesh (0.0 0.0 0.0) false)
  (`self.K2_SetActorLocation` (`self.Origin`) false true))

(fn `UserConstructionScript`
  (bind _meshes (`self.Meshes`))
  (bind _meshes_2 (`self.Meshes`))
  (bind _meshes_3 (`self.Meshes`))
  (bind _meshes_4 (`self.Meshes`))
  (bind _meshes_5 (`self.Meshes`))
  (bind _meshes_6 (`self.Meshes`))
  (bind _meshes_7 (`self.Meshes`))
  (`StaticMeshComponent.SetStaticMesh` (`self.StaticMesh`) (`|GetArrayItem` (`self.Meshes`) (`self.IndexMesh`)))
  (switch `int` (`KismetMathLibrary.RandomInteger` 7)
    (:`0`
      (set `self.ObjectType` "NewEnumerator0")
      (set `self.Repaired?` true)
      (`KismetArrayLibrary.Array_Clear` _meshes_5)
      (for _ (range 3)
        (`KismetArrayLibrary.Array_Add` _meshes_5 "/Game/Assets/Tools/cles.cles")))
    (:`1`
      (set `self.ObjectType` "NewEnumerator1")
      (set `self.Repaired?` true)
      (`KismetArrayLibrary.Array_Clear` _meshes_6)
      (for _ (range 3)
        (`KismetArrayLibrary.Array_Add` _meshes_6 "/Game/Assets/Tools/Chalumeau.Chalumeau")))
    (:`2`
      (set `self.ObjectType` "NewEnumerator2")
      (set `self.Repaired?` true)
      (`KismetArrayLibrary.Array_Clear` _meshes_7)
      (for _ (range 3)
        (`KismetArrayLibrary.Array_Add` _meshes_7 "/Game/Assets/Tools/Extincteur.Extincteur")))
    (:`3`
      (set `self.ObjectType` "NewEnumerator3")
      (set `self.RepairObject` "NewEnumerator0")
      (`KismetArrayLibrary.Array_Clear` _meshes)
      (`KismetArrayLibrary.Array_Add` _meshes "/Game/Assets/Props_Degradation/Batterie/props_degradé_batterie_Low.props_degradé_batterie_Low")
      (`KismetArrayLibrary.Array_Add` _meshes "/Game/Assets/Props_Degradation/Batterie/props_degradé_batterie_Mid.props_degradé_batterie_Mid")
      (`KismetArrayLibrary.Array_Add` _meshes "/Game/Assets/Props_Degradation/Batterie/props_degradé_batterie_Neuve.props_degradé_batterie_Neuve"))
    (:`4`
      (set `self.ObjectType` "NewEnumerator4")
      (set `self.RepairObject` "NewEnumerator0")
      (`KismetArrayLibrary.Array_Clear` _meshes_2)
      (`KismetArrayLibrary.Array_Add` _meshes_2 "/Game/Assets/Props_Degradation/Radar/props_degradé_radar_Low.props_degradé_radar_Low")
      (`KismetArrayLibrary.Array_Add` _meshes_2 "/Game/Assets/Props_Degradation/Radar/props_degradé_radar_Mid.props_degradé_radar_Mid")
      (`KismetArrayLibrary.Array_Add` _meshes_2 "/Game/Assets/Props_Degradation/Radar/props_degradé_radar_Neuve.props_degradé_radar_Neuve"))
    (:`5`
      (set `self.ObjectType` "NewEnumerator5")
      (set `self.RepairObject` "NewEnumerator1")
      (`KismetArrayLibrary.Array_Clear` _meshes_3)
      (`KismetArrayLibrary.Array_Add` _meshes_3 "/Game/Assets/Props_Degradation/Oxygene/props_degradé_o2_Low.props_degradé_o2_Low")
      (`KismetArrayLibrary.Array_Add` _meshes_3 "/Game/Assets/Props_Degradation/Oxygene/props_degradé_o2_Mid.props_degradé_o2_Mid")
      (`KismetArrayLibrary.Array_Add` _meshes_3 "/Game/Assets/Props_Degradation/Oxygene/props_degradé_o2_Neuve.props_degradé_o2_Neuve"))
    (:`6`
      (set `self.ObjectType` "NewEnumerator6")
      (set `self.RepairObject` "NewEnumerator0")
      (`KismetArrayLibrary.Array_Clear` _meshes_4)
      (`KismetArrayLibrary.Array_Add` _meshes_4 "/Game/Assets/Props_Degradation/Processeur/props_degradé_processeur_moteur_Low.props_degradé_processeur_moteur_Low")
      (`KismetArrayLibrary.Array_Add` _meshes_4 "/Game/Assets/Props_Degradation/Processeur/props_degradé_processeur_moteur_Mid.props_degradé_processeur_moteur_Mid")
      (`KismetArrayLibrary.Array_Add` _meshes_4 "/Game/Assets/Props_Degradation/Processeur/props_degradé_processeur_moteur_Neuve.props_degradé_processeur_moteur_Neuve"))))