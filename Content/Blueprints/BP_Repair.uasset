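; Repairable world object that fills a progress bar while being repaired and changes its mesh as the work advances.
; StartRepair and StopRepair toggle progress accumulation and post Wwise tool sound events, with the switch derived from the ObjectToRepair enum.
; Tick advances progress by RepairSpeed and uses DoOnce gates to show an intermediate mesh at halfway, then the final mesh at completion, hiding the widget and locking further repair.
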(event `self.ReceiveBeginPlay`
  (bind _aswg_repair_progress_bar (cast `/Game/Widgets/WG_RepairProgressBar` (`WidgetComponent.GetUserWidgetObject` (`self.Widget`))))
  (set `self.ProgressBar` (`/Game/Widgets/WG_RepairProgressBar.RepairProgress` _aswg_repair_progress_bar)))

(event `self.ReceiveTick`
  (params (DeltaSeconds :type "Float (single-precision)"))
  (if (not (`self.Repaired?`))
    (`|ExecutionSequence`
      (:`then_0`
        (if (`self.Repairing?`)
          (bind _output_get (set `self.RepairingProgress` (+ (* DeltaSeconds (`self.RepairSpeed`)) (`self.RepairingProgress`))))
          (`ProgressBar.SetPercent` (`self.ProgressBar`) _output_get)))
      (:`then_1`
        (if (>= (`self.RepairingProgress`) 1.0)
          (`/Engine/EditorBlueprintResources/StandardMacros.DoOnce` false
            (:`Completed`
              (`self.SwitchMesh` 2)
              (`SceneComponent.SetVisibility` (`self.Widget`) false false)
              (`self.StopRepair`)
              (set `self.Repaired?` true)))
          (elif (>= (`self.RepairingProgress`) 0.5)
            (`/Engine/EditorBlueprintResources/StandardMacros.DoOnce` false
              (:`Completed`
                (`self.SwitchMesh` 1)))))))))

(event `SwitchMesh`
  (params (Index :type Integer))
  (`StaticMeshComponent.SetStaticMesh` (`self.Sphere`) (`|GetArrayItem` (`self.Meshes`) Index)))

(event `StartRepair`
  (if (not (`self.Repaired?`))
    (set `self.Repairing?` true)
    (`AkGameplayStatics.SetSwitch` "Tools" (`KismetStringLibrary.Conv_StringToName` (`KismetStringLibrary.Replace` (`|GetEnumeratorNameAsString` (`self.ObjectToRepair`)) " " "_")) self)
    (`AkGameplayStatics.PostEvent` "/Game/Audio/Switch_Play_Tools.Switch_Play_Tools" self)))

(event `StopRepair`
  (set `self.Repairing?` false)
  (`AkGameplayStatics.PostEvent` "/Game/Audio/Switch_Stop_Tools.Switch_Stop_Tools" self))

(fn `UserConstructionScript`
  (`StaticMeshComponent.SetStaticMesh` (`self.Sphere`) (`|GetArrayItem` (`self.Meshes`))))