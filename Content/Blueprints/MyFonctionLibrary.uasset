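; Function library that mixes UI selection styling with random spawn-point picking.
; Button helpers swap the normal image and hide other states (their brightness change is unwired); text box helpers set background brightness.
; Spawn helpers scan a root's direct mesh children for floor or wall meshes, keeping each with 1-in-Rate odds (-1 uses a default).
; The breach variant also returns rotations, but clears only locations beforehand.
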(fn `Find_Locations_For_Spawn`
  (params (Root :type "SceneComponent Object Reference") (Rate :type Integer))
  (returns (NewParam :type "Array of Vector Structure"))
  (locals (Objects_Spawn_Rate :type Integer :default 20) (Locations_Of_Objects :type "Array of Vector Structure"))
  (`KismetArrayLibrary.Array_Clear` (`local.Locations_Of_Objects`))
  (for _array_element (`SceneComponent.GetChildrenComponents` Root false)
    (bind _asstatic_mesh_component (cast `StaticMeshComponent` _array_element))
    (if (== (`StaticMeshComponent.StaticMesh` _asstatic_mesh_component) "/Game/Assets/Basic/Basic_Sol.Basic_Sol")
      (if (== (`KismetMathLibrary.RandomInteger` (`KismetMathLibrary.SelectInt` (`local.Objects_Spawn_Rate`) Rate (== Rate -1))) 0)
        (`KismetArrayLibrary.Array_Add` (`local.Locations_Of_Objects`) (`SceneComponent.K2_GetComponentLocation` _array_element)))))
  (return (`local.Locations_Of_Objects`)))

(fn `Find_Locations_For_Spawn_Breaches`
  (params (Root :type "SceneComponent Object Reference") (Rate :type Integer))
  (returns (Locations :type "Array of Vector Structure") (Rotations :type "Array of Rotator Structure"))
  (locals (Locations_Of_Objects :type "Array of Vector Structure") (Wall_Meshes_Array :type "Array of StaticMesh Object Reference") (Objects_Spawn_Rate :type Integer :default 15) (Rotations_Of_Objects :type "Array of Rotator Structure"))
  (`KismetArrayLibrary.Array_Clear` (`local.Locations_Of_Objects`))
  (for _array_element (`SceneComponent.GetChildrenComponents` Root false)
    (bind _asstatic_mesh_component (cast `StaticMeshComponent` _array_element))
    (if (!= (`KismetArrayLibrary.Array_Find` (`local.Wall_Meshes_Array`) (`StaticMeshComponent.StaticMesh` _asstatic_mesh_component)) -1)
      (if (== (`KismetMathLibrary.RandomInteger` (`KismetMathLibrary.SelectInt` (`local.Objects_Spawn_Rate`) Rate (== Rate -1))) 0)
        (`KismetArrayLibrary.Array_Add` (`local.Locations_Of_Objects`) (`SceneComponent.K2_GetComponentLocation` _array_element))
        (`KismetArrayLibrary.Array_Add` (`local.Rotations_Of_Objects`) (`SceneComponent.K2_GetComponentRotation` _array_element)))))
  (return (`local.Locations_Of_Objects`) (`local.Rotations_Of_Objects`)))

(fn `SelectedButton`
  (params (Button :type "Button Object Reference") (`In Style Normal Image` :type "Object Object Reference"))
  (bind _widgetstyle_normal (break `ButtonStyle` (`Button.WidgetStyle` Button)))
  (`Button.SetStyle` Button (make `ButtonStyle` (make `SlateBrush` (`.ImageSize` (break `SlateBrush` _widgetstyle_normal)) (struct) (struct :`SpecifiedColor` (struct :`R` 1.0 :`G` 1.0 :`B` 1.0 :`A` 1.0) :`ColorUseRule` "UseColor_Specified") `In Style Normal Image`) (make `SlateBrush` (32.0 32.0) (struct) (make `SlateColor` (struct :`R` 1.0 :`B` 1.0)) null "NoDrawType") (make `SlateBrush` (32.0 32.0) (struct) (make `SlateColor` (struct :`R` 1.0 :`B` 1.0)) null "NoDrawType") (make `SlateBrush` (32.0 32.0) (struct) (make `SlateColor` (struct :`R` 1.0 :`B` 1.0)) null "NoDrawType"))))

(fn `SelectedTextBox`
  (params (TextBox :type "EditableTextBox Object Reference"))
  (bind _widgetstyle_backgroundimagenormal (break `EditableTextBoxStyle` (`EditableTextBox.WidgetStyle` TextBox)))
  (`KismetMathLibrary.LinearColor_SetFromHSV` (`.SpecifiedColor` (break `SlateColor` (`.TintColor` (break `SlateBrush` _widgetstyle_backgroundimagenormal)))) 0.0 0.0 0.2))

(fn `UnselectedButton`
  (params (Button :type "Button Object Reference") (`In Style Normal Image` :type "Object Object Reference"))
  (bind _widgetstyle_normal (break `ButtonStyle` (`Button.WidgetStyle` Button)))
  (`Button.SetStyle` Button (make `ButtonStyle` (make `SlateBrush` (`.ImageSize` (break `SlateBrush` _widgetstyle_normal)) (struct) (struct :`SpecifiedColor` (struct :`R` 1.0 :`G` 1.0 :`B` 1.0 :`A` 1.0) :`ColorUseRule` "UseColor_Specified") `In Style Normal Image`) (make `SlateBrush` (32.0 32.0) (struct) (make `SlateColor` (struct :`R` 1.0 :`B` 1.0)) null "NoDrawType") (make `SlateBrush` (32.0 32.0) (struct) (make `SlateColor` (struct :`R` 1.0 :`B` 1.0)) null "NoDrawType") (make `SlateBrush` (32.0 32.0) (struct) (make `SlateColor` (struct :`R` 1.0 :`B` 1.0)) null "NoDrawType"))))

(fn `UnselectedTextBox`
  (params (TextBox :type "EditableTextBox Object Reference"))
  (bind _widgetstyle_backgroundimagenormal (break `EditableTextBoxStyle` (`EditableTextBox.WidgetStyle` TextBox)))
  (`KismetMathLibrary.LinearColor_SetFromHSV` (`.SpecifiedColor` (break `SlateColor` (`.TintColor` (break `SlateBrush` _widgetstyle_backgroundimagenormal)))) 0.0 0.0 1.0))