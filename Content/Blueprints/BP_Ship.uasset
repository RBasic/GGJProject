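; Ship manager actor that runs the survival loop: oxygen, hull health, timed jumps and win/lose screens.
; Tick drains O2 per breach against life-support regen, damages GameInstance ShipHealth each second, toggles the Chameleon alarm and clears fires at low O2.
; Every 60-second jump tallies damage, then has BP_Generation spawn events scaled by jump count.
; Health also drives an audio RTPC; zero O2 or health means defeat, target score means victory.
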(event `self.ReceiveBeginPlay`
  ;[1 1 1] Seulement pour tester, a changer
  (`self.Start_Game`)
  (bind _outactors (`GameplayStatics.GetAllActorsOfClass` "/Script/Engine.PointLight"))
  (set `self.AllLightsLevel` _outactors)
  (bind _outactors_2 (`GameplayStatics.GetAllActorsOfClass` "/Game/Chameleon/Chameleon.Chameleon_C"))
  (set `self.RefChameleon` (`|GetArrayItem` _outactors_2)))

(event `Start_Game`
  (set `self.Time_Until_Next_Jump` 60.0)
  (set `self.Playtime` 0.0)
  (bind _outactors (`GameplayStatics.GetAllActorsOfClass` "/Game/Blueprints/BP_Placement.BP_Placement_C"))
  (for _array_element _outactors
    (`BlueprintMapLibrary.Map_Add` (`self.Systems_Map`) (`/Game/Blueprints/BP_Placement.System_Type` _array_element) _array_element))
  (bind _outactors_2 (`GameplayStatics.GetAllActorsOfClass` "/Game/Blueprints/BP_Generation.BP_Generation_C"))
  (bind _output_get (set `self.My_Generation` (`|GetArrayItem` _outactors_2)))
  (set `/Game/Blueprints/BP_Generation.My_Ship` self _output_get)
  (`/Game/Blueprints/BP_Generation.Jump` _output_get)
  (`/Game/Blueprints/BP_Generation.Generate_Events` _output_get (* (`self.Number_Of_Jump`) 4))
  (`/Game/Blueprints/BP_Generation.Spawn_Damages` _output_get))

(event `self.ReceiveTick`
  (params (DeltaSeconds :type "Float (single-precision)"))
  (bind _check_damage_tick (`self.Check_Damage_Tick`))
  (bind _asmy_game_instance (cast `/Game/GameManager/MyGameInstance` (`GameplayStatics.GetGameInstance`) :!pure true))
  (bind _asmy_game_instance_2 (cast `/Game/GameManager/MyGameInstance` (`GameplayStatics.GetGameInstance`) :!pure true))
  (bind _ship_health (`/Game/GameManager/MyGameInstance.Ship_Health` _asmy_game_instance))
  (`|ExecutionSequence`
    (:`then_0`
      (set `self.Playtime` (+ DeltaSeconds (`self.Playtime`)))
      (set `self.O2` (`KismetMathLibrary.FClamp` (+ (- (`self.O2`) (* (* (`self.Cptr_Breach`) (`self.O2_Loosing_Speed`)) DeltaSeconds)) (* (`KismetMathLibrary.SelectFloat` 0.0 (* (`self.Number_Of_Life_System`) (`self.Life_System_Efficiency`)) (`/Game/Blueprints/BP_Placement.Is_Broken?` (`BlueprintMapLibrary.Map_Find` (`self.Systems_Map`) "NewEnumerator1"))) DeltaSeconds)) 0.0 100.0))
      (bind _output_get (set `self.Time_Until_Next_Jump` (- (`self.Time_Until_Next_Jump`) DeltaSeconds)))
      (`|ExecutionSequence`
        (:`then_0`
          (if (<= _output_get 0.0)
            (`self.Initiate_Jump`)))
        (:`then_1`
          (if (< (`self.O2`) 50.0)
            (`self.SetAlarm` true)
            (else
              (`self.SetAlarm` false))))))
    (:`then_1`
      (set `self.Check_Damage_Tick` (+ DeltaSeconds _check_damage_tick))
      (if (>= _check_damage_tick 1.0)
        (set `self.Check_Damage_Tick` 0.0)
        (for _array_element (`self.My_Systems`)
          (if (`/Game/Blueprints/BP_Placement.Is_Broken?` _array_element)
            (set `/Game/GameManager/MyGameInstance.Ship_Health` (- _ship_health (`self.Damage_Per_System`)) _asmy_game_instance)))
        (set `/Game/GameManager/MyGameInstance.Ship_Health` (- _ship_health (* (`KismetMathLibrary.Conv_IntToDouble` (+ (`self.Cptr_Breach`) (`self.Cptr_Fire`))) (`self.Damage_Per_Cleanable`))) _asmy_game_instance)))
    (:`then_2`
      (if (or (<= (`self.O2`) 0.0) (<= (`/Game/GameManager/MyGameInstance.Ship_Health` (cast `/Game/GameManager/MyGameInstance` (`GameplayStatics.GetGameInstance`) :!pure true)) 0.0))
        (`self.Defeat` :!label _label)))
    (:`then_3`
      (if (>= (`/Game/GameManager/MyGameInstance.Current_Score` _asmy_game_instance_2) (`/Game/GameManager/MyGameInstance.Minimum_Score_To_Win` _asmy_game_instance_2))
        (`self.Victory`)))
    (:`then_4`
      (if (< (`self.O2`) 30.0)
        (`/Engine/EditorBlueprintResources/StandardMacros.DoOnce` false :!label _label_2
          (:`Completed`
            (bind _outactors (`GameplayStatics.GetAllActorsOfClass` "/Game/Blueprints/BP_Cleanable.BP_Cleanable_C"))
            (for _array_element_2 _outactors
              (if (`|EnumEquality` (`/Game/Blueprints/BP_Cleanable.Cleanable_Type` _array_element_2) "NewEnumerator1")
                (`self.K2_DestroyActor` _array_element_2)))))
        (else
          (goto _label_2 :!via `Reset`))))
    (:`then_5`
      (`AkGameplayStatics.SetRTPCValue` "Time" (- 100.0 (`/Game/GameManager/MyGameInstance.Ship_Health` (cast `/Game/GameManager/MyGameInstance` (`GameplayStatics.GetGameInstance`) :!pure true)))))))

(event `Initiate_Jump`
  (bind _my_generation (`self.My_Generation`))
  (bind _my_generation_2 (`self.My_Generation`))
  (`self.Check_Amount_Of_Damage`)
  (if (<= (`/Game/GameManager/MyGameInstance.Ship_Health` (cast `/Game/GameManager/MyGameInstance` (`GameplayStatics.GetGameInstance`) :!pure true)) 0.0)
    (goto _label)
    (else
      (set `self.Time_Until_Next_Jump` 60.0)
      (`/Engine/EditorBlueprintResources/StandardMacros.IncrementInt` (`self.Number_Of_Jump`)
        (:`  `
          (set `/Game/Blueprints/BP_Generation.Percent_Event_1` 0 _my_generation)
          (set `/Game/Blueprints/BP_Generation.Percent_Event_2` 0 _my_generation)
          (set `/Game/Blueprints/BP_Generation.Percent_Event_3` 0 _my_generation)
          (set `/Game/Blueprints/BP_Generation.Percent_Event_4` 0 _my_generation)
          (set `/Game/Blueprints/BP_Generation.Percent_Event_5` 0 _my_generation)
          (`/Game/Blueprints/BP_Generation.Generate_Events` _my_generation_2 (* (`self.Number_Of_Jump`) 4))
          (`/Game/Blueprints/BP_Generation.Spawn_Damages` _my_generation_2))))))

(event `SetLevelLight`
  (params (Multiplicateur :type Integer) (`Augmenter?` :type Boolean))
  (for _array_element (`self.AllLightsLevel`)
    (if `Augmenter?`
      (bind _pointlightcomponent (`PointLight.PointLightComponent` _array_element))
      (bind _intensity (`LightComponentBase.Intensity` _pointlightcomponent))
      (`LightComponent.SetIntensity` _pointlightcomponent (* Multiplicateur _intensity))
      (else
        (`LightComponent.SetIntensity` _pointlightcomponent (/ _intensity (`KismetMathLibrary.Conv_IntToDouble` Multiplicateur)))))))

(event `Check_Amount_Of_Damage`
  (set `self.Cptr_Breach` 0)
  (set `self.Cptr_Fire` 0)
  (set `self.Cptr_Damage_This_Round` 0)
  (bind _outactors (`GameplayStatics.GetAllActorsOfClass` "/Game/Blueprints/BP_Cleanable.BP_Cleanable_C"))
  (for _array_element _outactors
    (switch `/Game/Blueprints/Enum_Cleanable` (`/Game/Blueprints/BP_Cleanable.Cleanable_Type` _array_element)
      (:`NewEnumerator0`
        (`/Engine/EditorBlueprintResources/StandardMacros.IncrementInt` (`self.Cptr_Breach`)))
      (:`NewEnumerator1`
        (`/Engine/EditorBlueprintResources/StandardMacros.IncrementInt` (`self.Cptr_Fire`)))))
  (if (> (`self.Cptr_Breach`) 0)
    (`/Engine/EditorBlueprintResources/StandardMacros.IncrementInt` (`self.Cptr_Damage_This_Round`)
      (:`  `
        _)))
  (if (> (`self.Cptr_Fire`) 0)
    (`/Engine/EditorBlueprintResources/StandardMacros.IncrementInt` (`self.Cptr_Damage_This_Round`)
      (:`  `
        _)))
  (bind _outactors_2 (`GameplayStatics.GetAllActorsOfClass` "/Game/Blueprints/BP_Placement.BP_Placement_C"))
  (for _array_element_2 _outactors_2
    (if (`/Game/Blueprints/BP_Placement.Is_Broken?` _array_element_2)
      (`/Engine/EditorBlueprintResources/StandardMacros.IncrementInt` (`self.Cptr_Damage_This_Round`))))
  (bind _asmy_game_instance (cast `/Game/GameManager/MyGameInstance` (`GameplayStatics.GetGameInstance`)))
  (set `/Game/GameManager/MyGameInstance.Ship_Health` (- (`/Game/GameManager/MyGameInstance.Ship_Health` _asmy_game_instance) (`KismetMathLibrary.Conv_IntToDouble` (`self.Cptr_Damage_This_Round`))) _asmy_game_instance))

(event `Defeat`
  (set `/Game/GameManager/MyGameInstance.Win?` false (cast `/Game/GameManager/MyGameInstance` (`GameplayStatics.GetGameInstance`) :!pure true))
  (bind _returnvalue (`|CreateWidget` "/Game/Widgets/WG_Ending_Screen.WG_Ending_Screen_C"))
  (`UserWidget.AddToViewport` _returnvalue 0)
  (`GameplayStatics.SetGamePaused` true))

(event `Victory`
  (set `/Game/GameManager/MyGameInstance.Win?` true (cast `/Game/GameManager/MyGameInstance` (`GameplayStatics.GetGameInstance`) :!pure true))
  (bind _returnvalue (`|CreateWidget` "/Game/Widgets/WG_Ending_Screen.WG_Ending_Screen_C"))
  (`UserWidget.AddToViewport` _returnvalue 0)
  (`GameplayStatics.SetGamePaused` true))

(fn `SetAlarm`
  (params (`Alarm?` :type Boolean))
  (bind _refchameleon (`self.RefChameleon`))
  (if `Alarm?`
    (set `/Game/Chameleon/Chameleon.Alarm` true _refchameleon)
    (else
      (set `/Game/Chameleon/Chameleon.Alarm` false _refchameleon)))
  (return))

(fn `UserConstructionScript`)