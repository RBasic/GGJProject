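; Generates a ship's failures, hazards and repair tools around FTL-style jumps.
; Generate_Events raises five capped event chances using random team-name letters, while Jump sets one random chance to 80.
; Spawn_Objects resets repairable items, rolls those chances to break systems, spawns fires and breaches per room, and places one tool in each of the first three rooms.
; Five BP_Room grid layouts remain, apparently obsolete, with Generate_Map empty.
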(event `Map_1`
  (bind _scale (defaults `/Game/Blueprints/BP_Room` "/Game/Blueprints/BP_Room.BP_Room_C"))
  (bind (_x _y) (`KismetMathLibrary.BreakVector2D` (`self.Decalage_Initial`)))
  (bind _returnvalue (* _scale 100.0))
  ;[1 1 1] Obsolete
  (for _index (range 1 (+ (- (`self.Length`) 2) 1))
    (for _index_2 (range 1 (+ (- (`self.Height`) 2) 1))
      (`|SpawnActorFromClass` "/Game/Blueprints/BP_Room.BP_Room_C" (`KismetMathLibrary.MakeTransform` (`KismetMathLibrary.MakeVector` (+ (* _index_2 _returnvalue) _x) (+ _y (* _index _returnvalue)) (`self.Z`)) (struct) (`KismetMathLibrary.Conv_DoubleToVector` _scale)) "Undefined" "OverrideRootScale" null null))))

(event `Map_2`
  (bind _scale (defaults `/Game/Blueprints/BP_Room` "/Game/Blueprints/BP_Room.BP_Room_C"))
  (bind _returnvalue (- (`self.Length`) 1))
  (bind _returnvalue_2 (- (`self.Height`) 1))
  (bind (_x _y) (`KismetMathLibrary.BreakVector2D` (`self.Decalage_Initial`)))
  (bind _returnvalue_3 (* _scale 100.0))
  ;[1 1 1] Obsolete
  (for _index (range (+ _returnvalue 1))
    (for _index_2 (range (+ _returnvalue_2 1))
      (if (or (== _index 0) (== _index _returnvalue) (== _index_2 0) (== _index_2 _returnvalue_2))
        (`|SpawnActorFromClass` "/Game/Blueprints/BP_Room.BP_Room_C" (`KismetMathLibrary.MakeTransform` (`KismetMathLibrary.MakeVector` (+ (* _index_2 _returnvalue_3) _x) (+ _y (* _index _returnvalue_3)) (`self.Z`)) (struct) (`KismetMathLibrary.Conv_DoubleToVector` _scale)) "Undefined" "OverrideRootScale" null null)))))

(event `Map_3`
  (bind _scale (defaults `/Game/Blueprints/BP_Room` "/Game/Blueprints/BP_Room.BP_Room_C"))
  (bind _returnvalue (- (`self.Length`) 1))
  (bind _returnvalue_2 (- (`self.Height`) 1))
  (bind (_x _y) (`KismetMathLibrary.BreakVector2D` (`self.Decalage_Initial`)))
  (bind _returnvalue_3 (* _scale 100.0))
  ;[1 1 1] Obsolete
  (for _index (range (+ _returnvalue 1))
    (if (and (!= _index 0) (!= _index _returnvalue))
      (for _index_2 (range (+ _returnvalue_2 1))
        (bind _returnvalue_4 (== _index 1))
        (bind _returnvalue_5 (== _index_2 0))
        (bind _returnvalue_6 (== _index_2 _returnvalue_2))
        (bind _returnvalue_7 (== _index (- _returnvalue 1)))
        (if (not (or (and _returnvalue_4 _returnvalue_5) (and _returnvalue_4 _returnvalue_6) (and _returnvalue_7 _returnvalue_5) (and _returnvalue_7 _returnvalue_6)))
          (`|SpawnActorFromClass` "/Game/Blueprints/BP_Room.BP_Room_C" (`KismetMathLibrary.MakeTransform` (`KismetMathLibrary.MakeVector` (+ (* _index_2 _returnvalue_3) _x) (+ _y (* _index _returnvalue_3)) (`self.Z`)) (struct) (`KismetMathLibrary.Conv_DoubleToVector` _scale)) "Undefined" "OverrideRootScale" null null))))))

(event `Map_4`
  (bind _scale (defaults `/Game/Blueprints/BP_Room` "/Game/Blueprints/BP_Room.BP_Room_C"))
  (bind (_x _y) (`KismetMathLibrary.BreakVector2D` (`self.Decalage_Initial`)))
  (bind _returnvalue (* _scale 100.0))
  ;[1 1 1] Obsolete
  (for _index (range (`self.Length`))
    (if (and (!= _index 2) (!= _index 3))
      (for _index_2 (range (`self.Height`))
        (`|SpawnActorFromClass` "/Game/Blueprints/BP_Room.BP_Room_C" (`KismetMathLibrary.MakeTransform` (`KismetMathLibrary.MakeVector` (+ (* _index_2 _returnvalue) _x) (+ _y (* _index _returnvalue)) (`self.Z`)) (struct) (`KismetMathLibrary.Conv_DoubleToVector` _scale)) "Undefined" "OverrideRootScale" null null)))))

(event `Map_5`
  (bind _scale (defaults `/Game/Blueprints/BP_Room` "/Game/Blueprints/BP_Room.BP_Room_C"))
  (bind _returnvalue (- (`self.Height`) 1))
  (bind (_x _y) (`KismetMathLibrary.BreakVector2D` (`self.Decalage_Initial`)))
  (bind _returnvalue_2 (* _scale 100.0))
  ;[1 1 1] Obsolete
  (for _index (range (`self.Length`))
    (for _index_2 (range (+ _returnvalue 1))
      (if (or (== _index 2) (== _index 3))
        (`|SpawnActorFromClass` "/Game/Blueprints/BP_Room.BP_Room_C" (`KismetMathLibrary.MakeTransform` (`KismetMathLibrary.MakeVector` (+ (* _index_2 _returnvalue_2) _x) (+ _y (* _index _returnvalue_2)) (`self.Z`)) (struct) (`KismetMathLibrary.Conv_DoubleToVector` _scale)) "Undefined" "OverrideRootScale" null null :!label _label)
        (elif (and (or (== _index 0) (== _index 1)) (== _index_2 0))
          (goto _label)
          (elif (and (== _index_2 _returnvalue) (or (== _index 4) (== _index 5)))
            (goto _label)))))))

(event `Generate_Map`)

(event `self.ReceiveBeginPlay`)

(event `Generate_Events`
  (params (Number_Of_Jumps :type Integer))
  (bind _returnvalue (`KismetStringLibrary.GetCharacterArrayFromString` (`self.Team_Name`)))
  (bind _output (`|GetArrayItem` _returnvalue (`self.Random_Event`)))
  (for _ (range (+ (+ Number_Of_Jumps 3) 1))
    (set `self.Random_Event` (`KismetMathLibrary.RandomInteger` (`KismetArrayLibrary.Array_Length` _returnvalue)))
    (if (!= (`KismetArrayLibrary.Array_Find` (`self.Map_1_Characters`) _output) -1)
      (`self.Breche_Et_Survie`)
      (elif (!= (`KismetArrayLibrary.Array_Find` (`self.Map_2_Characters`) _output) -1)
        (`self.Feu_Et_Panne_Moteur`)
        (elif (!= (`KismetArrayLibrary.Array_Find` (`self.Map_3_Characters`) _output) -1)
          (`self.Fuites_D'Eau_Et_Processeur`)
          (elif (!= (`KismetArrayLibrary.Array_Find` (`self.Map_4_Characters`) _output) -1)
            (`self.Coupure_De_Courant`)
            (elif (!= (`KismetArrayLibrary.Array_Find` (`self.Map_5_Characters`) _output) -1)
              (`self.Radar_et_Armes`))))))))

(event `Jump`
  (set `self.Epreuve` (`KismetMathLibrary.RandomInteger` 5))
  (switch `int` (`self.Epreuve`)
    (:`0`
      (set `self.Percent_Event_1` 80))
    (:`1`
      (set `self.Percent_Event_2` 80))
    (:`2`
      (set `self.Percent_Event_3` 80))
    (:`3`
      (set `self.Percent_Event_4` 80))
    (:`4`
      (set `self.Percent_Event_5` 80))))

(event `Breche_Et_Survie`
  (set `self.Percent_Event_1` (`KismetMathLibrary.Clamp` (+ (`self.Percent_Event_1`) (`self.Taux_Par_Jump`)) 0 80)))

(event `Feu_Et_Panne_Moteur`
  (set `self.Percent_Event_2` (`KismetMathLibrary.Clamp` (+ (`self.Percent_Event_2`) (`self.Taux_Par_Jump`)) 0 80)))

(event `Fuites_D'Eau_Et_Processeur`
  (set `self.Percent_Event_3` (`KismetMathLibrary.Clamp` (+ (`self.Percent_Event_3`) (`self.Taux_Par_Jump`)) 0 80)))

(event `Radar_et_Armes`
  (set `self.Percent_Event_4` (`KismetMathLibrary.Clamp` (+ (`self.Percent_Event_4`) (`self.Taux_Par_Jump`)) 0 80)))

(event `Coupure_De_Courant`
  (set `self.Percent_Event_5` (`KismetMathLibrary.Clamp` (+ (`self.Percent_Event_5`) (`self.Taux_Par_Jump`)) 0 80)))

(event `Spawn_Objects`
  (bind _outactors (`GameplayStatics.GetAllActorsOfClass` "/Game/Blueprints/BP_Object.BP_Object_C"))
  (for _array_element _outactors
    (switch `/Game/Blueprints/Enum_Tools` (`/Game/Blueprints/BP_Object.ObjectType` _array_element)
      (:`NewEnumerator3`
        (set `/Game/Blueprints/BP_Object.Repaired?` false _array_element)
        (set `/Game/Blueprints/BP_Object.IndexMesh` 0 _array_element))
      (:`NewEnumerator4`
        (set `/Game/Blueprints/BP_Object.Repaired?` false _array_element)
        (set `/Game/Blueprints/BP_Object.IndexMesh` 0 _array_element))
      (:`NewEnumerator5`
        (set `/Game/Blueprints/BP_Object.Repaired?` false _array_element)
        (set `/Game/Blueprints/BP_Object.IndexMesh` 0 _array_element))
      (:`NewEnumerator6`
        (set `/Game/Blueprints/BP_Object.Repaired?` false _array_element)
        (set `/Game/Blueprints/BP_Object.IndexMesh` 0 _array_element)))
    (`/Game/Blueprints/BP_Object.Init_Objects` _array_element))
  (bind _outactors_2 (`GameplayStatics.GetAllActorsOfClass` "/Game/Blueprints/BP_Placement.BP_Placement_C"))
  (for _array_element_2 _outactors_2
    (switch `/Game/Blueprints/Enum_System_Name` (`/Game/Blueprints/BP_Placement.System_Type` _array_element_2)
      (:`NewEnumerator0`
        (if (<= (`KismetMathLibrary.RandomInteger` 100) (`KismetMathLibrary.Max` (`self.Percent_Event_2`) (`self.Percent_Event_4`)))
          (set `/Game/Blueprints/BP_Placement.Is_Broken?` true _array_element_2 :!label _label_2)
          (else
            (`/Game/Blueprints/BP_Placement.Destroy_Particle` _array_element_2 :!label _label_3))))
      (:`NewEnumerator1`
        (if (<= (`KismetMathLibrary.RandomInteger` 100) (`self.Percent_Event_1`))
          (goto _label_2)
          (else
            (goto _label_3))))
      (:`NewEnumerator2`
        (if (<= (`KismetMathLibrary.RandomInteger` 100) (`self.Percent_Event_5`))
          (goto _label_2)
          (else
            (goto _label_3))))
      (:`NewEnumerator3`
        (if (<= (`KismetMathLibrary.RandomInteger` 100) (`self.Percent_Event_3`))
          (goto _label_2)
          (else
            (goto _label_3))))
      (:`NewEnumerator4`
        (if (<= (`KismetMathLibrary.RandomInteger` 100) (`self.Percent_Event_4`))
          (goto _label_2)
          (else
            (goto _label_3))))))
  (set `self.Cptr` 0)
  (for (_array_element_3 _array_index) (`self.Room_Classes_Array`)
    (bind _outactors_3 (`GameplayStatics.GetAllActorsOfClass` _array_element_3))
    (bind _rootcomponent (`Actor.RootComponent` (`|GetArrayItem` _outactors_3)))
    (`self.Spawn_Cleanable` _rootcomponent)
    (if (<= _array_index 2)
      (bind _newparam (`/Game/Blueprints/MyFonctionLibrary.Find_Locations_For_Spawn` _rootcomponent))
      (bind _returnvalue (`|SpawnActorFromClass` "/Game/Blueprints/BP_Object.BP_Object_C" (`KismetMathLibrary.MakeTransform` (`|GetArrayItem` _newparam (`KismetMathLibrary.RandomInteger` (`KismetArrayLibrary.Array_Length` _newparam)))) "Undefined" "OverrideRootScale" null null))
      (set `/Game/Blueprints/BP_Object.ObjectType` (select `int` (`self.Cptr`) :`0` "NewEnumerator0" :`1` "NewEnumerator1" :`2` "NewEnumerator2" :!type "/Game/Blueprints/Enum_Tools Enum") _returnvalue)
      (set `/Game/Blueprints/BP_Object.Repaired?` true _returnvalue)
      (bind _meshes (`/Game/Blueprints/BP_Object.Meshes` _returnvalue))
      (`KismetArrayLibrary.Array_Clear` _meshes)
      (for _ (range 3)
        (`KismetArrayLibrary.Array_Add` _meshes (select `int` (`self.Cptr`) :`0` "/Game/Assets/Tools/cles.cles" :`1` "/Game/Assets/Tools/Chalumeau.Chalumeau" :`2` "/Game/Assets/Tools/Extincteur.Extincteur" :!type "StaticMesh Object Reference")))
      (`/Game/Blueprints/BP_Object.Init_Objects` _returnvalue)
      (`/Engine/EditorBlueprintResources/StandardMacros.IncrementInt` (`self.Cptr`)))))

(fn `Spawn_Cleanable`
  (params (Root :type "SceneComponent Object Reference"))
  (bind _newparam (`/Game/Blueprints/MyFonctionLibrary.Find_Locations_For_Spawn` Root (`KismetMathLibrary.FTrunc` (/ (`KismetMathLibrary.Conv_IntToDouble` (- 100 (`self.Percent_Event_2`))) 2.0))))
  (for _array_element _newparam
    (bind _returnvalue (`|SpawnActorFromClass` "/Game/Blueprints/BP_Cleanable.BP_Cleanable_C" (`KismetMathLibrary.MakeTransform` (+ _array_element (0.0 0.0 70.0))) "Undefined" "OverrideRootScale" null null))
    (set `/Game/Blueprints/BP_Cleanable.Cleanable_Type` "NewEnumerator1" _returnvalue)
    (set `/Game/Blueprints/BP_Cleanable.Repair_Object` "NewEnumerator2" _returnvalue)
    (`/Game/Blueprints/BP_Cleanable.Init_Particles` _returnvalue))
  (bind (_locations _rotations) (`/Game/Blueprints/MyFonctionLibrary.Find_Locations_For_Spawn_Breaches` Root (`KismetMathLibrary.FTrunc` (/ (`KismetMathLibrary.Conv_IntToDouble` (- 100 (`self.Percent_Event_1`))) 2.0))))
  (for (_array_element_2 _array_index) _locations
    (bind _returnvalue_2 (`|SpawnActorFromClass` "/Game/Blueprints/BP_Cleanable.BP_Cleanable_C" (`KismetMathLibrary.MakeTransform` (+ _array_element_2 (0.0 0.0 70.0)) (`|GetArrayItem` _rotations _array_index)) "Undefined" "OverrideRootScale" null null))
    (set `/Game/Blueprints/BP_Cleanable.Cleanable_Type` "NewEnumerator0" _returnvalue_2)
    (set `/Game/Blueprints/BP_Cleanable.Repair_Object` "NewEnumerator1" _returnvalue_2)
    (`/Game/Blueprints/BP_Cleanable.Init_Particles` _returnvalue_2)))

(fn `UserConstructionScript`)