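; BP_Concombre is a playable cucumber character Blueprint that builds on a parent class with grab and power mechanics.
; After the parent Tick, it lowers walk speed while a valid GrabbedObject is held and restores it otherwise.
; Pressing Power posts a Wwise speed-effect sound and spawns a splash actor at the mesh location, pitched with random yaw; the handler itself changes no speed.
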(event `self.ReceiveTick`
  (params (DeltaSeconds :type "Float (single-precision)"))
  (bind _charactermovement (`self.CharacterMovement`))
  (`parent.ReceiveTick` DeltaSeconds)
  ;[1 1 1] PlayerMovement Grabbing
  (`/Engine/EditorBlueprintResources/StandardMacros.IsValid` (`self.GrabbedObject`)
    (:`Is Valid`
      (set `CharacterMovementComponent.MaxWalkSpeed` 300.0 _charactermovement))
    (:`Is Not Valid`
      (set `CharacterMovementComponent.MaxWalkSpeed` 900.0 _charactermovement))))

(event `InputAction|Power`
  (params (Key :type "Key Structure"))
  (:`Pressed`
    (`AkGameplayStatics.PostEvent` "/Game/Audio/Play_SFX_speedEffect_cornichon.Play_SFX_speedEffect_cornichon" self)
    (`|SpawnActorFromClass` "/Game/Blueprints/M_Splash_Inst_Blueprint.M_Splash_Inst_Blueprint_C" (`KismetMathLibrary.MakeTransform` (`SceneComponent.K2_GetComponentLocation` (`self.Mesh`)) (`KismetMathLibrary.MakeRotator` 0.0 90.0 (`KismetMathLibrary.RandomFloatInRange` 0.0 360.0))) "Undefined" "OverrideRootScale" null null)))

(fn `UserConstructionScript`
  (`parent.UserConstructionScript`))