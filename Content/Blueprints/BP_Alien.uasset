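; Playable alien character that spawns an egg at BeginPlay and uses it as a movable teleport anchor.
; A short tap of the Power input moves the egg to the alien, while holding it for the full timer teleports the alien to the egg.
; Tick advances the hold timer, shown through a dynamic material on the progress widget, and reduces walk speed while grabbing an object.
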(event `self.ReceiveBeginPlay`
  ;[1 1 1] get ref widget
  (bind _returnvalue (`|SpawnActorFromClass` "/Game/Blueprints/BP_Egg.BP_Egg_C" (`KismetMathLibrary.MakeTransform` (`self.K2_GetActorLocation`)) "Undefined" "OverrideRootScale" null null))
  (set `self.Egg` _returnvalue)
  (bind _returnvalue_2 (`Image.GetDynamicMaterial` (`/Game/Widgets/WG_ProgressBarAlien.Image_113` (cast `/Game/Widgets/WG_ProgressBarAlien` (`WidgetComponent.GetUserWidgetObject` (`self.Widget`)) :!pure true))))
  (set `self.ProgressMat` _returnvalue_2))

(event `self.ReceiveTick`
  (params (DeltaSeconds :type "Float (single-precision)"))
  (bind _charactermovement (`self.CharacterMovement`))
  (`parent.ReceiveTick` DeltaSeconds)
  (`|ExecutionSequence`
    (:`then_0`
      ;[1 1 1] PlayerMovement if grabbing
      (`/Engine/EditorBlueprintResources/StandardMacros.IsValid` (`self.GrabbedObject`)
        (:`Is Valid`
          (set `CharacterMovementComponent.MaxWalkSpeed` 300.0 _charactermovement))
        (:`Is Not Valid`
          (set `CharacterMovementComponent.MaxWalkSpeed` 600.0 _charactermovement))))
    (:`then_1`
      ;[1 1 1] Teleport egg
      (if (`self.Pressed?`)
        (set `self.Timer` (+ DeltaSeconds (`self.Timer`)))
        (`MaterialInstanceDynamic.SetScalarParameterValue` (`self.ProgressMat`) "Alpha" (/ (`self.Timer`) (`self.TimerMax`)))
        (if (>= (`self.Timer`) (`self.TimerMax`))
          (`self.K2_SetActorLocation` (`self.K2_GetActorLocation` (`self.Egg`)) false true)
          (set `self.Pressed?` false)
          (set `self.Timer` 0.0)
          (`MaterialInstanceDynamic.SetScalarParameterValue` (`self.ProgressMat`) "Alpha" 0.0))))))

(event `InputAction|Power`
  (params (Key :type "Key Structure"))
  ;[1 1 1] Input Power Alien
  (:`Pressed`
    (set `self.Pressed?` true))
  (:`Released`
    (if (`self.Pressed?`)
      (set `self.Pressed?` false)
      (if (<= (`self.Timer`) 0.5)
        (`self.K2_SetActorLocation` (`self.Egg`) (`self.K2_GetActorLocation`) false true))
      (`MaterialInstanceDynamic.SetScalarParameterValue` (`self.ProgressMat`) "Alpha" 0.0)
      (set `self.Timer` 0.0))))

(fn `UserConstructionScript`
  (`parent.UserConstructionScript`))