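; BP_Cleanable is a ship hazard, either a breach or a fire, that is removed by repairing it over time.
; Init_Particles applies the decal, particle and Wwise audio matching its type.
; While repairing, Tick advances progress and shows it on a widget bar, and start/stop events switch tool sounds based on RepairObject.
; On completion it decrements the matching BP_Ship counter and destroys itself.
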(event `Init_Particles`
  (switch `/Game/Blueprints/Enum_Cleanable` (`self.Cleanable_Type`)
    (:`NewEnumerator0`
      (`DecalComponent.SetDecalMaterial` (`self.Breach_Material`) "/Game/Decals/Breach/M_Decal_Breach_Inst.M_Decal_Breach_Inst")
      (`ParticleSystemComponent.SetTemplate` (`self.Breach_Particle`) "/Game/particule/blackHole.blackHole")
      (`AkGameplayStatics.PostEvent` "/Game/Audio/event_Ship/event_faille.event_faille" self))
    (:`NewEnumerator1`
      (`ParticleSystemComponent.SetTemplate` (`self.Fire_Particle`) "/Game/Particles/Fire_ball/P_Fire.P_Fire")
      (`AkGameplayStatics.PostEvent` "/Game/Audio/event_Ship/Play_SFX_Fire_loop.Play_SFX_Fire_loop" self))))

(event `self.ReceiveBeginPlay`
  (bind _aswg_repair_progress_bar (cast `/Game/Widgets/WG_RepairProgressBar` (`WidgetComponent.GetUserWidgetObject` (`self.WG Progress Bar`))))
  (set `self.ProgressBar` (`/Game/Widgets/WG_RepairProgressBar.RepairProgress` _aswg_repair_progress_bar))
  (bind _outactors (`GameplayStatics.GetAllActorsOfClass` "/Game/Blueprints/BP_Ship.BP_Ship_C"))
  (set `self.My_Ship` (`|GetArrayItem` _outactors)))

(event `self.ReceiveTick`
  (params (DeltaSeconds :type "Float (single-precision)"))
  (bind _my_ship (`self.My_Ship`))
  (`|ExecutionSequence`
    (:`then_0`
      (`/Engine/EditorBlueprintResources/StandardMacros.IsValid` (`self.ProgressBar`)
        (:`Is Valid`
          (`SceneComponent.SetVisibility` (`self.WG Progress Bar`) (`self.Repairing?`) false))))
    (:`then_1`
      (if (`self.Repairing?`)
        (bind _output_get (set `self.RepairingProgress` (+ (* DeltaSeconds (`self.RepairSpeed`)) (`self.RepairingProgress`))))
        (`ProgressBar.SetPercent` (`self.ProgressBar`) _output_get)))
    (:`then_2`
      (if (>= (`self.RepairingProgress`) 1.0)
        (`/Engine/EditorBlueprintResources/StandardMacros.DoOnce` false
          (:`Completed`
            (`self.StopRepair`)
            (switch `/Game/Blueprints/Enum_Cleanable` (`self.Cleanable_Type`)
              (:`NewEnumerator0`
                (`/Engine/EditorBlueprintResources/StandardMacros.DecrementInt` (`/Game/Blueprints/BP_Ship.Number_Of_Small_Breach` _my_ship)
                  (:`  `
                    _)))
              (:`NewEnumerator1`
                (`/Engine/EditorBlueprintResources/StandardMacros.DecrementInt` (`/Game/Blueprints/BP_Ship.Number_Of_Fires` _my_ship)
                  (:`  `
                    _))))
            (`self.K2_DestroyActor`)))))))

(event `StartRepair`
  (set `self.Repairing?` true)
  (`AkGameplayStatics.SetSwitch` "Tools" (`KismetStringLibrary.Conv_StringToName` (`KismetStringLibrary.Replace` (`|GetEnumeratorNameAsString` (`self.Repair_Object`)) " " "_" "CaseSensitive")) self)
  (`AkGameplayStatics.PostEvent` "/Game/Audio/character/Switch_Play_Tools.Switch_Play_Tools" self))

(event `StopRepair`
  (set `self.Repairing?` false)
  (`AkGameplayStatics.PostEvent` "/Game/Audio/character/Switch_Stop_Tools.Switch_Stop_Tools" self))

(fn `UserConstructionScript`)