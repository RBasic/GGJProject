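; BP_Placement is a placement spot that, while broken, tracks a BP_Object in its box and consumes it once repair completes.
; Box overlap stores one object at a time and posts a Wwise tools sound switched by the expected type; end overlap clears it.
; Tick destroys the stored object when its repair progress is full and its type matches ObjectToPlace.
; IsBroken is only read here, never changed.
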(event `self.ReceiveTick`
  (params (DeltaSeconds :type "Float (single-precision)"))
  (bind _objectref (`self.ObjectRef`))
  (`/Engine/EditorBlueprintResources/StandardMacros.IsValid` _objectref
    (:`Is Valid`
      (if (and (>= (`/Game/Blueprints/BP_Object.RepairingProgress` _objectref) 1.0) (`KismetStringLibrary.EqualEqual_StrStr` (`|GetEnumeratorNameAsString` (`/Game/Blueprints/BP_Object.ObjectType` _objectref)) (`|GetEnumeratorNameAsString` (`self.ObjectToPlace`))) (`self.Is_Broken?`))
        (`self.K2_DestroyActor` _objectref)))))

(event `self.Box.OnComponentBeginOverlap`
  (params (OverlappedComponent :type "PrimitiveComponent Object Reference") (OtherActor :type "Actor Object Reference") (OtherComp :type "PrimitiveComponent Object Reference") (OtherBodyIndex :type Integer) (bFromSweep :type Boolean) (SweepResult :type "HitResult Structure (by ref)"))
  (if (`self.Is_Broken?`)
    (`/Engine/EditorBlueprintResources/StandardMacros.IsValid` (`self.ObjectRef`)
      (:`Is Not Valid`
        (bind _asbp_object (cast `/Game/Blueprints/BP_Object` OtherActor))
        (set `self.ObjectRef` _asbp_object)
        (`AkGameplayStatics.SetSwitch` "ToolsEvent" (`KismetStringLibrary.Conv_StringToName` (`|GetEnumeratorNameAsString` (`self.ObjectToPlace`))) self)
        (`AkGameplayStatics.PostEvent` "/Game/Audio/Play_ToolsEvent.Play_ToolsEvent" self)))))

(event `self.Box.OnComponentEndOverlap`
  (params (OverlappedComponent :type "PrimitiveComponent Object Reference") (OtherActor :type "Actor Object Reference") (OtherComp :type "PrimitiveComponent Object Reference") (OtherBodyIndex :type Integer))
  (if (and (== OtherActor (`self.ObjectRef`)) (`self.Is_Broken?`))
    (set `self.ObjectRef` null)))

(fn `UserConstructionScript`)